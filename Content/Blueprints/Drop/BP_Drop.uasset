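; BP_Drop is a world item pickup that spawns with a random rotation and adds itself to the player's inventory when interacted with.
; On BeginPlay it looks up ItemID in the game mode's ItemsList to set its child actor mesh, then enables physics and attaches an interactable component.
; A one-second polling loop disables physics once velocity exceeds 1 with PhysicsOptimization enabled.
; Interaction passes ItemID and ItemValue to BP_Comp_Inventory and destroys the drop.
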(event Custom|OnInteract
  (bind _itemid (Variables|Default|GetItemID))
  (bind _itemvalue (Variables|Default|GetItemValue))
  (bind _st_inv_item (Utilities|Struct|MakeST_Inv_Item "00000000000000000000000000000000" _itemid _itemvalue))
  (bind _error (Default|FindIteminDB (Variables|Default|GetItemsList) _st_inv_item))
  (if (not _error)
    (Default|AddItem (Actor|GetComponentbyClass (Game|Player|GetPlayerPawn 0) "/Game/Blueprints/Inventory/BP_Comp_Inventory.BP_Comp_Inventory_C") _st_inv_item)
    (Actor|DestroyActor)))

(event EventBeginPlay
  (bind _childactor (Variables|Default|GetChildActor))
  (bind _childactor_2 (Variables|/Script/Engine.ChildActorComponent|GetChildActor _childactor))
  (Transformation|SetActorRotation (Math|Random|RandomRotator true))
  (bind _asbp_first_person_game_mode (Utilities|Casting|CastToBP_FirstPersonGameMode (Game|GetGameMode)))
  (bind _output_get (Variables|Default|SetItemsList (Variables|/Game/Blueprints/BP_FirstPersonGameMode.BP_FirstPersonGameMode_C|GetItemsList _asbp_first_person_game_mode)))
  (bind (_output _error) (Default|FindIteminDB _output_get (Utilities|Struct|MakeST_Inv_Item "00000000000000000000000000000000" (Variables|Default|GetItemID))))
  (if (not _error)
    (ChildActorComponent|SetChildActorClass (Variables|Default|GetChildActor) (.Mesh (Utilities|Struct|BreakST_DB_Item _output)))
    (Variables|Default|SetWeaponCollider (Actor|GetComponentbyClass _childactor_2 "/Script/Engine.StaticMeshComponent"))
    (Collision|SetCollisionEnabled (Variables|Default|GetWeaponCollider) "QueryAndPhysics")
    (Physics|SetSimulatePhysics (Variables|Default|GetWeaponCollider) true)
    (bind _returnvalue (AddComponent|AddBPCompInteractable _childactor_2))
    (EventDispatchers|BindEventtoOnInteract _returnvalue (delegate Custom|OnInteract))
    (Variables|Default|SetPhysicsComponent (Actor|GetComponentbyClass (Variables|/Script/Engine.ChildActorComponent|GetChildActor (Variables|Default|GetChildActor)) "/Script/Engine.StaticMeshComponent"))
    (bind _returnvalue_2 (CallFunction|GetVel))
    (if (and (> _returnvalue_2 1.0) (Variables|Default|GetPhysicsOptimization)) :!label _label
      (Physics|SetSimulatePhysics (Variables|Default|GetPhysicsComponent) false)
      (else
        (Utilities|FlowControl|Delay 1.0)
        (goto _label)))))

(fn ConstructionScript)

(fn GetVel
  (bind _physicscomponent (Variables|Default|GetPhysicsComponent))
  (return (Math|Vector|VectorLength (Transformation|GetComponentVelocity _physicscomponent)) _physicscomponent))