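; Inventory component that stores item stacks and tracks the selected active weapon slot.
; AddItem validates items against the game mode's item database, tops up matching stacks to their maximum, adds any remainder as a new GUID-tagged entry, then fires a change event.
; Slot selection clamps or wraps across three slots and broadcasts changes.
; ActiveItemGet resolves the slot's GUID, falling back to a default item; RemoveItem is an empty stub.
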(event EventBeginPlay
  (bind _asbp_first_person_game_mode (Utilities|Casting|CastToBP_FirstPersonGameMode (Game|GetGameMode)))
  (Variables|Default|SetItemsList (Variables|/Game/Blueprints/BP_FirstPersonGameMode.BP_FirstPersonGameMode_C|GetItemsList _asbp_first_person_game_mode)))

(fn AddItem
  (params (ItemValue :type ST%20Inv%20Item%20Structure))
  (bind _output_get (LocalVariables|SetAddedItem ItemValue))
  (bind (_output _error) (CallFunction|FindIteminDB _output_get))
  (LocalVariables|SetCurrentItemID (.ItemID (Utilities|Struct|BreakST_Inv_Item (LocalVariables|GetAddedItem))))
  (if (not _error)
    (LocalVariables|SetMaxValue (.MaxValue (Utilities|Struct|BreakST_DB_Item _output)))
    (for (_array_element _array_index) (Variables|Default|GetInventoryList)
      (LocalVariables|SetArrayIndex _array_index)
      (bind _returnvalue (CallFunction|IsItemsSame _array_element (LocalVariables|GetAddedItem)))
      (LocalVariables|SetArrayItem _array_element)
      (if _returnvalue
        (bind _iscanadd (CallFunction|IsCanAddInstack (LocalVariables|GetArrayItem) (LocalVariables|GetMaxValue) (LocalVariables|GetAddedItem)))
        (if _iscanadd
          (while (and (> (.Value (Utilities|Struct|BreakST_Inv_Item (LocalVariables|GetAddedItem))) 0) (< (.Value (Utilities|Struct|BreakST_Inv_Item (LocalVariables|GetArrayItem))) (LocalVariables|GetMaxValue)))
            (bind _structout (Utilities|Struct|SetmembersinST_Inv_Item (LocalVariables|GetAddedItem) (- (.Value (Utilities|Struct|BreakST_Inv_Item (LocalVariables|GetAddedItem))) 1)))
            (LocalVariables|SetAddedItem _structout)
            (bind _structout_2 (Utilities|Struct|SetmembersinST_Inv_Item (LocalVariables|GetArrayItem) (+ (.Value (Utilities|Struct|BreakST_Inv_Item (LocalVariables|GetArrayItem))) 1)))
            (Utilities|Array|SetArrayElem (Variables|Default|GetInventoryList) (LocalVariables|GetArrayIndex) _structout_2)))))
    (if (> (.Value (Utilities|Struct|BreakST_Inv_Item (LocalVariables|GetAddedItem))) 0)
      (Utilities|Array|Add (Variables|Default|GetInventoryList) (Utilities|Struct|MakeST_Inv_Item (Guid|NewGuid) (.ItemID (Utilities|Struct|BreakST_Inv_Item (LocalVariables|GetAddedItem))) (.Value (Utilities|Struct|BreakST_Inv_Item (LocalVariables|GetAddedItem))))))
    (Default|CallOnInventroyChanged)))

(fn RemoveItem)

(fn FindIteminDB
  (params (Item :type ST%20Inv%20Item%20Structure))
  (bind (_output _error) (Default|FindIteminDB (Variables|Default|GetItemsList) Item))
  (return _output _error))

(fn IsCanAddInstack
  (params (CurrentItem :type ST%20Inv%20Item%20Structure%20%28by%20ref%29) (MaxValue :type Integer) (AddItem :type ST%20Inv%20Item%20Structure))
  (return MaxValue (< (.Value (Utilities|Struct|BreakST_Inv_Item CurrentItem)) MaxValue)))

(fn IsItemsSame
  (params (It1 :type ST%20Inv%20Item%20Structure%20%28by%20ref%29) (It2 :type ST%20Inv%20Item%20Structure))
  (return (== (.ItemID (Utilities|Struct|BreakST_Inv_Item It2)) (.ItemID (Utilities|Struct|BreakST_Inv_Item It1)))))

(fn GetInventoryList
  (return (Variables|Default|GetInventoryList)))

(fn ActiveItemSelect
  (params (WeaponIndex :type Integer))
  (bind _output_get (Variables|Default|SetSelectedItem (Math|Integer|Clamp(Integer) WeaponIndex 0 2)))
  (Default|CallOnChangeSelectedWeapon _output_get))

(fn ActiveItemAddValue
  (params (AddVal :type Integer))
  (bind _output_get (Variables|Default|SetSelectedItem (+ (Variables|Default|GetSelectedItem) AddVal)))
  (if (>= _output_get (Utilities|Array|Length (Variables|Default|GetActiveList)))
    (Variables|Default|SetSelectedItem 0))
  (if (< (Variables|Default|GetSelectedItem) 0)
    (Variables|Default|SetSelectedItem 2))
  (CallFunction|ActiveItemSelect (Variables|Default|GetSelectedItem)))

(fn ActiveItemGet
  (bind _st_inv_item (Utilities|Struct|MakeST_Inv_Item "00000000000000000000000000000000" 2))
  (bind _activelist (Variables|Default|GetActiveList))
  (bind _selecteditem (Variables|Default|GetSelectedItem))
  (bind _output (Utilities|Array|Get(acopy) _activelist _selecteditem))
  (if (== _output (Utilities|Struct|MakeGuid))
    (bind (_output_2 _error) (CallFunction|FindIteminDB _st_inv_item :!label _label))
    (if (not _error)
      (return _st_inv_item _output_2))
    (else
      (bind _array_element (Utilities|Array|ForEachLoopwithBreak (Variables|Default|GetInventoryList))
        (:LoopBody
          (if (== (.UID (Utilities|Struct|BreakST_Inv_Item _array_element)) _output)
            (bind (_output_3 _error_2) (CallFunction|FindIteminDB _array_element))
            (if (not _error_2)
              (return _array_element _output_3))))
        (:Completed
          (goto _label))))))