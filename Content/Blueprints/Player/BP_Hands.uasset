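; Player hands Blueprint that carries a weapon and adds procedural motion to the skeletal mesh.
; Each tick it lerps mesh rotation toward a mouse-delta-driven sway.
; It also line-traces forward from an Arrow against WorldStatic objects, easing the mesh along local Y by the blocked distance to handle wall clipping.
; SetWeaponActor swaps the child actor class from a database item and copies its weapon data into the weapon component.
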(event EventTick
  (params (DeltaSeconds :type Float%20%28single-precision%29))
  (CallFunction|HandsAnimations DeltaSeconds)
  (CallFunction|HandsClipping 1.3e+02 DeltaSeconds))

(event EventBeginPlay
  (Variables|Default|SetPlayer (Game|GetPlayerController 0)))

(fn ConstructionScript)

(fn HandsAnimations
  (params (Delta :type Float%20%28double-precision%29))
  (bind _player (Variables|Default|GetPlayer))
  (bind _skeletalmesh (Variables|Default|GetSkeletalMesh))
  (bind (_deltax _deltay) (Class|PlayerController|GetInputMouseDelta _player))
  (Transformation|SetRelativeRotation _skeletalmesh (Math|Rotator|Lerp(Rotator) (Variables|/Script/Engine.SceneComponent|GetRelativeRotation _skeletalmesh) (* (Math|Rotator|MakeRotator _deltay 0.0 _deltax) (Variables|Default|GetAngleStrength)) (* Delta (Variables|Default|GetRotateSpeed)) true) false false))

(fn HandsClipping
  (params (Distance :type Float%20%28double-precision%29) (DeltaTime :type Float%20%28double-precision%29))
  (bind _arrow (Variables|Default|GetArrow))
  (bind _skeletalmesh (Variables|Default|GetSkeletalMesh))
  (bind _returnvalue (Transformation|GetWorldLocation _arrow))
  (LocalVariables|SetDist Distance)
  (LocalVariables|SetDelta DeltaTime)
  (bind (_outhit _returnvalue_2) (Collision|LineTraceForObjects _returnvalue (+ (* (Math|Vector|GetForwardVector _arrow) (LocalVariables|GetDist)) _returnvalue) (Utilities|Array|MakeArray "ObjectTypeQuery1") false 0 "None"))
  (if _returnvalue_2
    (LocalVariables|SetNextPos (Math|Vector|MakeVector 0.0 (- (LocalVariables|GetDist) (.distance _outhit)) 0.0))
    (else
      (LocalVariables|SetNextPos "0, 0, 0")))
  (Transformation|SetRelativeLocation _skeletalmesh (Math|Vector|Lerp(Vector) (Variables|/Script/Engine.SceneComponent|GetRelativeLocation _skeletalmesh) (LocalVariables|GetNextPos) (* (LocalVariables|GetDelta) (Variables|Default|GetClipSpeed))) false false))

(fn SetWeaponActor
  (params (InvItem :type ST%20Inv%20Item%20Structure) (DBItem :type ST%20DB%20Item%20Structure))
  (bind (_itemtype _actor _mesh _maxvalue _weapondata) (Utilities|Struct|BreakST_DB_Item DBItem))
  (bind _weaponactor (Variables|Default|GetWeaponActor))
  (bind _childactor (Variables|/Script/Engine.ChildActorComponent|GetChildActor _weaponactor))
  (bind _returnvalue (Actor|GetComponentbyClass _childactor "/Game/Items/Weapons/BP_Comp_Weapon.BP_Comp_Weapon_C"))
  (ChildActorComponent|SetChildActorClass (Variables|Default|GetWeaponActor) _actor)
  (Development|PrintString "Hello")
  (Utilities|IsValid _returnvalue
    (:Is%20Valid
      (Variables|/Game/Items/Weapons/BP_Comp_Weapon.BP_Comp_Weapon_C|SetWeaponData _returnvalue (|Copy _weapondata)))))