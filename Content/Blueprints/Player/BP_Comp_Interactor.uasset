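; BP_Comp_Interactor is a player component that lets the player interact with world objects carrying a BP_Comp_Interactable component.
; A shared LineTrace casts a short object-type ray forward from the supplied camera against static, dynamic and physics-body objects.
; Interact calls InteractObject on the hit actor's interactable, passing the hit component.
; UpdateInteractState uses the same trace to set IsCanInteract according to whether an interactable is in view.
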(event EventBeginPlay
  (bind _object_types (Variables|Default|GetObject%20Types))
  (Utilities|Array|Add _object_types "ObjectTypeQuery1")
  (Utilities|Array|Add _object_types "ObjectTypeQuery2")
  (Utilities|Array|Add _object_types "ObjectTypeQuery4"))

(fn Interact
  (params (Camera :type Camera%20Component%20Object%20Reference))
  (bind (_outhit _returnvalue) (CallFunction|LineTrace Camera))
  (if _returnvalue
    (Utilities|IsValid (Actor|GetComponentbyClass (.HitActor (Collision|BreakHitResult _outhit)) "/Game/Enviroment/BP/Components/BP_Comp_Interactable.BP_Comp_Interactable_C")
      (:Is%20Valid
        (Default|InteractObject (Actor|GetComponentbyClass (.HitActor (Collision|BreakHitResult _outhit)) "/Game/Enviroment/BP/Components/BP_Comp_Interactable.BP_Comp_Interactable_C") (.HitComponent (Collision|BreakHitResult _outhit)))))))

(fn LineTrace
  (params (Camera :type Scene%20Component%20Object%20Reference))
  (bind _returnvalue (Transformation|GetWorldLocation Camera))
  (bind (_outhit _returnvalue_2) (Collision|LineTraceForObjects _returnvalue (+ _returnvalue (* (Math|Vector|GetForwardVector Camera) (Math|Float|MakeLiteralFloat 3.5e+02))) (Variables|Default|GetObject%20Types) false 0 "None"))
  (return _outhit _returnvalue_2))

(fn UpdateInteractState
  (params (Camera :type Camera%20Component%20Object%20Reference))
  (bind (_outhit _returnvalue) (CallFunction|LineTrace Camera))
  (if _returnvalue
    (Utilities|IsValid (Actor|GetComponentbyClass (.HitActor (Collision|BreakHitResult _outhit)) "/Game/Enviroment/BP/Components/BP_Comp_Interactable.BP_Comp_Interactable_C")
      (:Is%20Valid
        (Variables|Default|SetIsCanInteract true))
      (:Is%20Not%20Valid
        (Variables|Default|SetIsCanInteract false :!label _label)))
    (else
      (goto _label))))