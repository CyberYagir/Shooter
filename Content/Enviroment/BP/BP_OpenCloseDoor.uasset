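; BP_OpenCloseDoor is an interactable door that swings its Arrow component between open and closed rotations.
; BPCompInteractable's interact event enables Tick for one second, during which PartOCTweenRotate rotates the Arrow at the component's animation speed.
; Child primitive collision is set from the current opened state when motion starts.
; After the delay, Tick stops, the opened state inverts and collision is reset with a fixed true state.
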(event Custom|OnInteract
  (Actor|Tick|SetActorTickEnabled true)
  (CallFunction|CollisiontoOpened)
  (Utilities|FlowControl|Delay 1.0)
  (Actor|Tick|SetActorTickEnabled false)
  (Default|OpenedInvert (Variables|Default|GetBP_Comp_Interactable))
  (CallFunction|CollisionState true))

(event EventBeginPlay
  (EventDispatchers|BindEventtoOnInteract (Variables|Default|GetBP_Comp_Interactable) (delegate Custom|OnInteract))
  (Actor|Tick|SetActorTickEnabled false))

(event EventTick
  (params (DeltaSeconds :type Float%20%28single-precision%29))
  (bind _bp_comp_interactable (Variables|Default|GetBP_Comp_Interactable))
  (CallFunction|PartOCTweenRotate (Variables|Default|GetArrow) (* DeltaSeconds (Variables|/Game/Enviroment/BP/Components/BP_Comp_Interactable.BP_Comp_Interactable_C|GetAnimationSpeed _bp_comp_interactable)) (Variables|Default|GetRotator%20Open) (Variables|Default|GetRotator%20Close) (Variables|/Game/Enviroment/BP/Components/BP_Comp_Interactable.BP_Comp_Interactable_C|GetIsOpened _bp_comp_interactable) (Variables|Default|GetShortestPath)))

(fn ConstructionScript)

(fn CollisiontoOpened
  (CallFunction|CollisionState (Variables|/Game/Enviroment/BP/Components/BP_Comp_Interactable.BP_Comp_Interactable_C|GetIsOpened (Variables|Default|GetBP_Comp_Interactable))))

(fn CollisionState
  (params (IsOpen :type Boolean))
  (for _array_element (Components|GetChildrenComponents (Variables|Default|GetDefaultSceneRoot) true)
    (bind _asprimitive_component (Utilities|Casting|CastToPrimitiveComponent _array_element))
    (CallFunction|PartOCEnableCollision _asprimitive_component IsOpen)))