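; BP_Env_Methods provides helper functions for environment parts that switch between open and closed states.
; PartOCTweenRotate lerps from the part's current relative rotation by a supplied alpha, targeting the close rotator when IsOpen is true and the open rotator otherwise, with optional shortest path.
; PartOCEnableCollision sets a primitive to query and physics collision when IsOpen is true and to no collision otherwise.
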(fn PartOCTweenRotate
  (params (Mesh :type Scene%20Component%20Object%20Reference) (Alpha :type Float%20%28single-precision%29) (RotatorOpen :type Rotator) (RotatorClose :type Rotator) (IsOpen :type Boolean) (ShortestPath :type Boolean))
  (LocalVariables|SetTransform Mesh)
  (if IsOpen
    (LocalVariables|SetCurrentRotator RotatorClose)
    (else
      (LocalVariables|SetCurrentRotator RotatorOpen)))
  (Transformation|SetRelativeRotation (LocalVariables|GetTransform) (Math|Rotator|Lerp(Rotator) (Variables|/Script/Engine.SceneComponent|GetRelativeRotation (LocalVariables|GetTransform)) (LocalVariables|GetCurrentRotator) Alpha ShortestPath) false false))

(fn PartOCEnableCollision
  (params (Primitive :type Primitive%20Component%20Object%20Reference) (IsOpen :type Boolean))
  (if IsOpen
    (Collision|SetCollisionEnabled Primitive "QueryAndPhysics")
    (else
      (Collision|SetCollisionEnabled Primitive "NoCollision")))
  (return))